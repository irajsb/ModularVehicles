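; Blueprint for a Chieftain MK6 modular tank, whose own logic lives entirely in the construction script.
; It positions six left and six right wheel components from the bones of the skeletal mesh.
; It then passes the left wheels and two idlers to a single TankTrack component to set up the track.
; BeginPlay and Tick are empty.
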(event EventTick
  (params (DeltaSeconds :type Float%20%28single-precision%29)))

(event EventBeginPlay)

(fn ConstructionScript
  (Class|ModularVehicleFunctionLibrary|SetupWheelLocationfromBone (Variables|Default|GetSkeletalMesh) (Utilities|Array|MakeArray (Variables|Default|GetL_06) (Variables|Default|GetR_05) (Variables|Default|GetR_04) (Variables|Default|GetR_03) (Variables|Default|GetR_02) (Variables|Default|GetR_01) (Variables|Default|GetR_06) (Variables|Default|GetL_05) (Variables|Default|GetL_01) (Variables|Default|GetL_04) (Variables|Default|GetL_03) (Variables|Default|GetL_02)))
  (Class|TankTrackComponent|SetupComponents (Variables|Default|GetTankTrack) (Utilities|Array|MakeArray (Variables|Default|GetL_06) (Variables|Default|GetL_05) (Variables|Default|GetL_04) (Variables|Default|GetL_03) (Variables|Default|GetL_02) (Variables|Default|GetL_01) (Variables|Default|GetIdler) (Variables|Default|GetIdler1))))