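; Semi truck vehicle Blueprint that adds trailer towing and engine effects to a parent vehicle built on ModularMovement.
; Tick drives two particle systems' strength from engine load or an interpolated cold-start value while the engine runs, and upshifts play a flutter sound.
; An input action triggers the trailer attach point; attach changes run a timeline that shifts the spring arm's offset and pitch limit.
; Physics sleep changes also propagate to the attached trailer.
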(event OnGearChange(ModularMovement)
  (params (CurrentGear :type Integer) (TargetGear :type Integer) (Finished :type Boolean))
  (if (and (not Finished) (> TargetGear CurrentGear))
    (Audio|PlaySoundatLocation "/Game/Art/Sound/Engine/FlutterHeavy/Flutter1_Cue.Flutter1_Cue" (Transformation|GetWorldLocation (Variables|Default|GetChasis)) "0, 0, 0" 1.0 1.0 0.0 0 0 0 0)))

(event OnSleepChange(ModularMovement)
  (params (Sleep :type Boolean))
  (Class|ModularMovementComponent|SetSleeponBody 0 Sleep)
  (bind _otherattachpoint (Variables|/Script/ModularMovement.TrailerAttachPoint|GetOtherAttachPoint (Variables|Default|GetBP_TrailerAttachPoint))
    (:then
      (bind _asprimitive_component (Utilities|Casting|CastToPrimitiveComponent (Variables|/Script/Engine.Actor|GetRootComponent (Components|GetOwner _otherattachpoint))))
      (Class|ModularMovementComponent|SetSleeponBody _asprimitive_component Sleep))
    (:else)))

(event OnTrailerAttach(BP_TrailerAttachPoint)
  (params (NewAttach :type Boolean) (FromSave :type Boolean) (ConstraintComponent :type Physics%20Constraint%20Component%20Object%20Reference))
  (if NewAttach
    (bind _newtrack_0 (Timeline|Timeline PlayFromStart)
      (:Update
        (Variables|/Script/ModularMovement.VehicleSpringArm|SetSocketOffset (Variables|Default|GetVehicleSpringArm) (Math|Vector|Lerp(Vector) "0, 0, 0" "-333.333333,0.000000,100.000000" _newtrack_0))
        (Variables|/Script/ModularMovement.VehicleSpringArm|SetMinPitch (Variables|Default|GetVehicleSpringArm) (Math|Float|Lerp 1e+01 -5.0 _newtrack_0))))
    (else
      (Timeline|Timeline ReverseFromEnd))))

(event Collision|EventActorBeginOverlap
  (params (OtherActor :type Actor%20Object%20Reference))
  (|CallParentFunction OtherActor) ; This node is disabled and will not be called.\nDrag off pins to build functionality.
)

(event EventTick
  (params (DeltaSeconds :type Float%20%28single-precision%29))
  (bind _modularmovement (Variables|Default|GetModularMovement))
  (bind _vehiclestate (Variables|/Script/ModularMovement.ModularMovementComponent|GetVehicleState _modularmovement))
  (Utilities|FlowControl|Sequence
    (:then_0
      (if (.isengineon _vehiclestate)
        (Variables|Default|SetColdStart (Math|Interpolation|FInterptoConstant (Variables|Default|GetColdStart) 0.0 DeltaSeconds 1.0)))
      (|CallParentFunction DeltaSeconds)
      (Effects|Components|ParticleSystem|SetFloatParameter (Variables|Default|GetParticleSystem) "Strentgh" (Math|Float|SelectFloat (Math|Float|Max(Float) (Variables|/Script/ModularMovement.VehicleAudioComponent|GetLoad (Variables|Default|GetVehicleAudio)) (Variables|Default|GetColdStart)) 0.0 (.isengineon _vehiclestate))))))

(event EventBeginPlay
  (|CallParentFunction))

(event Input|ActionEvents|InputActionAction2
  (params (Key :type Key%20Structure :default "None"))
  (:Pressed
    (Class|TrailerAttachPoint|OnTrailerButtonPress (Variables|Default|GetBP_TrailerAttachPoint) false)))

(fn ConstructionScript
  (|CallParentFunction))