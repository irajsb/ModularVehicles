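; Solid-axle differential Blueprint for vehicles, pairing left and right wheels on one skeletal mesh axle.
; Setup constrains both wheels to the vehicle body as an axle, attaches suspension roots to it, and outside construction drops the axle by suspension length to rest.
; The construction script applies optional wheel mesh, scale and data overrides, mirroring the left mesh with negative Y scale.
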(event Custom|MoveToRestPosition
  (Transformation|SetWorldLocation (Variables|Default|GetSkeletalMesh) (- (Transformation|GetActorLocation) (Math|Vector|MakeVector 0.0 0.0 (Variables|/Script/ModularMovement.ModularVehicleWheelData|GetSuspensionLength (Class|ModularWheel|GetWheelSetup (Variables|Default|GetRight))))) false true))

(event Custom|DisableEffects)

(event EventBeginPlay)

(fn ConstructionScript
  (CallFunction|SetWheelOverrides)
  (bind _vehicle_wheel_dataoverride (Variables|Default|GetVehicle%20Wheel%20DataOverride)
    (:then
      (Class|ModularWheel|SetupWheelClass (Variables|Default|GetLeft) (Utilities|ResolveSoftReference _vehicle_wheel_dataoverride)))
    (:else)))

(fn Setup
  (params (Mesh :type Primitive%20Component%20Object%20Reference) (MC :type Modular%20Movement%20Component%20Object%20Reference) (FromConstruct :type Boolean))
  (Class|ModularWheel|SetupConstraints (Variables|Default|GetRight) MC Mesh (Variables|Default|GetSkeletalMesh) (Variables|Default|GetRightMesh) (Variables|Default|GetRConstraint) true)
  (Class|ModularWheel|SetupConstraints (Variables|Default|GetLeft) MC Mesh (Variables|Default|GetSkeletalMesh) (Variables|Default|GetLeftMesh) (Variables|Default|GetLConstraint) true)
  (Transformation|AttachComponentToComponent (Variables|Default|GetSuspRootL) Mesh "None" "KeepWorld" "KeepWorld" "KeepWorld" true)
  (Transformation|AttachComponentToComponent (Variables|Default|GetSuspRootR) Mesh "None" "KeepWorld" "KeepWorld" "KeepWorld" true)
  (if (not FromConstruct)
    (CallFunction|MovetoRestPosition)))

(fn SetWheelOverrides
  (bind _scaleoverride (Variables|Default|GetScaleOverride))
  (bind (_x _y _z) (Math|Vector|BreakVector _scaleoverride))
  (Utilities|FlowControl|Sequence
    (:then_0
      (bind _staticmeshoverride (Variables|Default|GetStaticMeshOverride)
        (:then
          (Components|StaticMesh|SetStaticMesh (Variables|Default|GetRightMesh) _staticmeshoverride)
          (Components|StaticMesh|SetStaticMesh (Variables|Default|GetLeftMesh) _staticmeshoverride)
          (Transformation|SetWorldScale3D (Variables|Default|GetRightMesh) _scaleoverride)
          (Transformation|SetWorldScale3D (Variables|Default|GetLeftMesh) (Math|Vector|MakeVector _x (* _y -1.0) _z)))
        (:else)))))