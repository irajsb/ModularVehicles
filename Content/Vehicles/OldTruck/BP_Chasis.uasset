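; Old truck chassis Blueprint that drives a ModularMovement vehicle, with starter control and a sleeping NPC mode.
; Construction and BeginPlay wire child-actor solid differentials to the chassis mesh and movement component.
; Tick broadcasts brake lights when throttle opposes gear direction and sets the tire audio speed parameter, then immediately fades it out.
; It also drives dynamic tire materials: pressure from wheel load, wetness and mud from surface physical materials.
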(event Custom|UpdateTirePressures
  (params (DeltaTime :type Float%20%28double-precision%29))
  ;[1 1 1] TirePressure
  (for _array_element (Actor|GetAllChildActors true)
    (for _array_element_2 (Actor|GetComponentsByClass _array_element "/Script/ModularMovement.ModularWheel")
      (Utilities|FlowControl|Sequence
        (:then_0
          (for _array_element_3 (Variables|/Script/ModularMovement.ModularWheel|GetChildWheels _array_element_2)
            (bind _asprimitive_component (Utilities|Casting|CastToPrimitiveComponent _array_element_3))
            (bind _asmaterial_instance_dynamic (Utilities|Casting|CastToMaterialInstanceDynamic (Rendering|Material|GetMaterial _asprimitive_component 0))
              (:then
                (bind _returnvalue (Rendering|Material|GetScalarParameterValue _asmaterial_instance_dynamic "Pressure" :!class /Script/Engine.MaterialInstanceDynamic))
                (Rendering|Material|SetScalarParameterValue _asmaterial_instance_dynamic "Pressure" (Math|Interpolation|FInterptoConstant _returnvalue (Math|Float|MapRangeClamped (Math|Vector|VectorLength (.WheelLoad (Utilities|Struct|BreakModularWheelState (Variables|/Script/ModularMovement.ModularWheel|GetWheelState _array_element_2)))) 0.0 (Variables|Default|GetMaxTireLoad) 1.0 0.5) DeltaTime 1.0) :!class /Script/Engine.MaterialInstanceDynamic))
              (:CastFailed
                (bind _returnvalue_2 (Rendering|Material|CreateDynamicMaterialInstance _asprimitive_component 0 (Rendering|Material|GetMaterial _asprimitive_component 0) "None" :!class /Script/Engine.PrimitiveComponent))
                (Rendering|Material|SetScalarParameterValue _returnvalue_2 "Pressure" (Math|Float|MapRangeClamped (Math|Vector|VectorLength (.WheelLoad (Utilities|Struct|BreakModularWheelState (Variables|/Script/ModularMovement.ModularWheel|GetWheelState _array_element_2)))) 0.0 (Variables|Default|GetMaxTireLoad) 1.0 0.5) :!class /Script/Engine.MaterialInstanceDynamic)))))
        (:then_1
          (for _array_element_4 (Variables|/Script/ModularMovement.ModularWheel|GetChildWheels _array_element_2)
            (bind _asprimitive_component_2 (Utilities|Casting|CastToPrimitiveComponent _array_element_4))
            (bind _asmaterial_instance_dynamic_2 (Utilities|Casting|CastToMaterialInstanceDynamic (Rendering|Material|GetMaterial _asprimitive_component_2 0)))
            (bind _returnvalue_3 (Rendering|Material|GetScalarParameterValue _asmaterial_instance_dynamic_2 "Wetness" :!class /Script/Engine.MaterialInstanceDynamic))
            (Rendering|Material|SetScalarParameterValue _asmaterial_instance_dynamic_2 "Wetness" (Math|Interpolation|FInterpTo _returnvalue_3 (Math|Conversions|ToFloat(Boolean) (== (Class|ModularWheel|GetActivePhysicalMaterial _array_element_2) "/Game/Assets/Materials/Physics/PA_WaterDrag.PA_WaterDrag")) DeltaTime (Math|Float|SelectFloat 15.0 0.05 (== (Class|ModularWheel|GetActivePhysicalMaterial _array_element_2) "/Game/Assets/Materials/Physics/PA_WaterDrag.PA_WaterDrag"))) :!class /Script/Engine.MaterialInstanceDynamic)
            (bind _returnvalue_4 (Rendering|Material|GetScalarParameterValue _asmaterial_instance_dynamic_2 "Mud" :!class /Script/Engine.MaterialInstanceDynamic))
            (Rendering|Material|SetScalarParameterValue _asmaterial_instance_dynamic_2 "Mud" (Math|Interpolation|FInterpTo _returnvalue_4 (Math|Conversions|ToFloat(Boolean) (== (Class|ModularWheel|GetActivePhysicalMaterial _array_element_2) "/Game/Assets/Materials/Physics/PA_MudDrag.PA_MudDrag")) DeltaTime (Math|Float|SelectFloat 0.5 0.25 (== (Class|ModularWheel|GetActivePhysicalMaterial _array_element_2) "/Game/Assets/Materials/Physics/PA_MudDrag.PA_MudDrag"))) :!class /Script/Engine.MaterialInstanceDynamic)))))))

(event Custom|SetNPCCar
  (Class|ModularMovementComponent|SetSleeping (Variables|Default|GetModularMovement) true)
  (for _array_element (Actor|GetComponentsByClass "/Script/Engine.ChildActorComponent")
    (bind _asbp_differential_solid (Utilities|Casting|CastToBP_Differential_Solid (Variables|/Script/Engine.ChildActorComponent|GetChildActor _array_element)))
    (Class|ModularWheel|DisableSurfaceEffects (Variables|/Game/Vehicles/SharedAssets/Bluepritns/Differentials/BP_Differential_Solid.BP_Differential_Solid_C|GetLeft _asbp_differential_solid))))

(event Custom|SetIdleBrakeInput
  (params (In :type Float%20%28double-precision%29))
  (Variables|/Script/ModularMovement.ModularVehicleData|SetIdleBrakeInput (Class|ModularMovementComponent|GetSetup (Variables|Default|GetModularMovement)) In))

(event Custom|CheckForBrakeLight
  (bind _modularmovement (Variables|Default|GetModularMovement))
  (bind _returnvalue (Class|ModularVehicleFunctionLibrary|GetGearBox _modularmovement))
  (bind _rawthrottleinput (Variables|/Script/ModularMovement.ModularMovementComponent|GetRawThrottleInput _modularmovement))
  (bind _returnvalue_2 (Math|Float|Sign(Float) _rawthrottleinput))
  ;[1 1 1] Brake Light
  (Default|CallOnBrakeLight (and (!= _returnvalue_2 0.0) (!= _returnvalue_2 (Class|KismetMathLibrary|SignOfInteger (- (Variables|/Script/ModularMovement.ModularGearBox|GetCurrentGear _returnvalue) (Variables|/Script/ModularMovement.ModularGearBox|GetIdleGear _returnvalue)))))))

(event Custom|UpdateTireSound
  (params (DeltaTime :type Float%20%28double-precision%29))
  (bind _tireaudio (Variables|Default|GetTireAudio))
  (Audio|Parameter|SetFloatParameter _tireaudio "Speed" (Math|Float|Absolute(Float) (/ (Math|Conversions|ToFloat(Integer) (Class|ModularVehicleFunctionLibrary|GetForwardSpeedKMH (Variables|Default|GetModularMovement))) 1e+02)) :!class /Script/AudioExtensions.AudioParameterControllerInterface)
  (Audio|Components|Audio|FadeOut _tireaudio 0.0 0.0 "Linear" :!class /Script/Engine.AudioComponent))

(event Custom|UpdateStarter
  (params (Down :type Boolean))
  (bind _modularmovement (Variables|Default|GetModularMovement))
  (if Down
    (if (.IsEngineOn (Utilities|Struct|BreakModularVehicleState (Variables|/Script/ModularMovement.ModularMovementComponent|GetVehicleState _modularmovement)))
      (Class|ModularMovementComponent|StopEngine _modularmovement)
      (else
        (Class|ModularMovementComponent|HoldStarter _modularmovement (Variables|Default|GetStartTime))))
    (else
      (Class|ModularMovementComponent|ReleaseStarter _modularmovement))))

(event EventBeginPlay
  (CallFunction|Initialize false))

(event EventTick
  (params (DeltaSeconds :type Float%20%28single-precision%29))
  (Utilities|FlowControl|Sequence
    (:then_0
      (CallFunction|CheckforBrakeLight)
      (CallFunction|UpdateTireSound DeltaSeconds)
      (CallFunction|UpdateTirePressures DeltaSeconds))))

(event Input|KeyboardEvents|DebugKeyR
  (params (Key :type Key%20Structure) (ActionValue :type Input%20Action%20Value%20Structure))
  (:Pressed
    (Class|ModularMovementComponent|HoldStarter (Variables|Default|GetModularMovement) 0.1)))

(fn ConstructionScript
  (CallFunction|Initialize true))

(fn Initialize
  (params (FromConstruct :type Boolean))
  (for _array_element (Actor|GetComponentsByClass "/Script/Engine.ChildActorComponent")
    (bind _asbp_differential_solid (Utilities|Casting|CastToBP_Differential_Solid (Variables|/Script/Engine.ChildActorComponent|GetChildActor _array_element)))
    (Utilities|FlowControl|Sequence
      (:then_0
        (Default|Setup _asbp_differential_solid (Variables|Default|GetChasis) (Variables|Default|GetModularMovement) FromConstruct))
      (:then_1))))