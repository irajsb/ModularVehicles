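; BP_Trailer is a towable semi-trailer built on a chassis with child-actor solid differentials.
; Construction and BeginPlay set up each differential with the chassis mesh and ModularMovement, and BeginPlay also overrides the left and right parent bodies.
; The attach-point event plays a timeline that moves the platform jacks, snapping them when restoring from a save.
; Detaching reverses the timeline, with constraint destruction handled on its completion.
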(event OnTrailerAttach(BP_TrailerAttachPoint)
  (params (NewAttach :type Boolean) (FromSave :type Boolean) (ConstraintComponent :type Physics%20Constraint%20Component%20Object%20Reference))
  (bind _trailer_semi_trailer_platform_jacks (Variables|Default|GetTrailer_Semi_Trailer_Platform_Jacks))
  (if NewAttach
    (Collision|SetCollisionEnabled (Variables|Default|GetTrailer_Semi_Trailer_Platform_Jacks) (select NewAttach "NoCollision" "PhysicsOnly"))
    (if FromSave
      (Transformation|SetRelativeLocation (Variables|Default|GetTrailer_Semi_Trailer_Platform_Jacks) "0.000000,0.000000,69.000000" false false)
      (else
        (bind _direction (Timeline|Timeline Play)
          (:Update
            (Transformation|AddRelativeLocation _trailer_semi_trailer_platform_jacks (Math|Vector|MakeVector 0.0 0.0 (Utilities|Select :Index _direction :Forward 1.0 :Backward -1.0)) false false))
          (:Finished
            (if (not NewAttach)
              (Class|PhysicsConstraintComponent|BreakConstraint ConstraintComponent)
              (Components|DestroyComponent ConstraintComponent)
              (Collision|SetCollisionEnabled _trailer_semi_trailer_platform_jacks "NoCollision"))))))
    (else
      (Timeline|Timeline ReverseFromEnd))))

(event EventBeginPlay
  (bind _chasis (Variables|Default|GetChasis))
  (Utilities|FlowControl|Sequence
    (:then_0
      (CallFunction|Initialize false)
      (for _array_element (Utilities|Array|MakeArray (Variables|Default|GetChildActor) (Variables|Default|GetChildActor1) (Variables|Default|GetChildActor2))
        (bind _asbp_differential_solid (Utilities|Casting|CastToBP_Differential_Solid (Variables|/Script/Engine.ChildActorComponent|GetChildActor _array_element)))
        (Variables|/Script/ModularMovement.ModularWheel|SetParentBodyOverride (Variables|/Game/Vehicles/SharedAssets/Bluepritns/Differentials/BP_Differential_Solid.BP_Differential_Solid_C|GetLeft _asbp_differential_solid) _chasis)
        (Variables|/Script/ModularMovement.ModularWheel|SetParentBodyOverride (Variables|/Game/Vehicles/SharedAssets/Bluepritns/Differentials/BP_Differential_Solid.BP_Differential_Solid_C|GetRight _asbp_differential_solid) _chasis)))))

(fn ConstructionScript
  (CallFunction|Initialize true))

(fn Initialize
  (params (FromConstruct :type Boolean))
  (for _array_element (Actor|GetComponentsByClass "/Script/Engine.ChildActorComponent")
    (bind _asbp_differential_solid (Utilities|Casting|CastToBP_Differential_Solid (Variables|/Script/Engine.ChildActorComponent|GetChildActor _array_element)))
    (Default|Setup _asbp_differential_solid (Variables|Default|GetChasis) (Variables|Default|GetModularMovement) FromConstruct)))

(fn ComponentstoSave
  (return 0))