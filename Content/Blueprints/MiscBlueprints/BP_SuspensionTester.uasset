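; BP_SuspensionTester is a test actor, apparently for vehicle suspension, that bobs its static mesh up and down.
; Tick accumulates elapsed time and sets the mesh's relative Z from a sine wave, scaled by the Frequency and Distance variables.
; The move is swept without teleporting, so blocking collision can stop the mesh along its path.
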(event EventBeginPlay)

(event Collision|EventActorBeginOverlap
  (params (OtherActor :type Actor%20Object%20Reference)))

(event EventTick
  (params (DeltaSeconds :type Float%20%28single-precision%29))
  (Variables|Default|SetTime (+ DeltaSeconds (Variables|Default|GetTime)))
  (Transformation|SetRelativeLocation (Variables|Default|GetStaticMesh) (Math|Vector|MakeVector 0.0 0.0 (* (Math|Trig|Sin(Radians) (* (Variables|Default|GetTime) (Variables|Default|GetFrequency))) (Variables|Default|GetDistance))) true false))

(fn ConstructionScript)