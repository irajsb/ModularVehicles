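; Spline-driven road actor that builds a chain of spline mesh segments along an editable path, with optional closed loop.
; The construction script divides the spline length by a segment length scaled by actor X scale, then adds one spline mesh component per step.
; Each segment takes local positions and tangents from the spline, with tangents clamped to segment length to limit distortion.
; The event graph has no active logic.
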(event EventBeginPlay)

(event Collision|EventActorBeginOverlap
  (params (OtherActor :type Actor%20Object%20Reference)))

(event EventTick
  (params (DeltaSeconds :type Float%20%28single-precision%29)))

(fn ConstructionScript
  (bind _spline (Variables|Default|GetSpline))
  (Spline|SetClosedLoop (Variables|Default|GetSpline) (Variables|Default|GetCloseLoop) true)
  (Variables|Default|SetCalculatedSegmentLen (* (Variables|Default|GetSegmentLen) (.x (Transformation|GetActorScale3D))))
  (for _index (range 0 (Math|Float|Truncate (/ (Spline|GetSplineLength (Variables|Default|GetSpline)) (Variables|Default|GetCalculatedSegmentLen))))
    (bind _returnvalue (AddComponent|AddSplineMeshComponent false (Math|Transform|MakeTransform "0, 0, 0" "0, 0, 0" "3.000000,3.000000,3.000000")))
    (SplineMesh|SetForwardAxis _returnvalue "X" true)
    (SplineMesh|SetStartandEnd _returnvalue (Spline|GetLocationatDistanceAlongSpline _spline (* _index (Variables|Default|GetCalculatedSegmentLen)) "Local") (Math|Vector|ClampVectorSize (Spline|GetTangentatDistanceAlongSpline _spline (* _index (Variables|Default|GetCalculatedSegmentLen)) "Local") 0.0 (Variables|Default|GetCalculatedSegmentLen)) (Spline|GetLocationatDistanceAlongSpline _spline (* (+ _index 1) (Variables|Default|GetCalculatedSegmentLen)) "Local") (Math|Vector|ClampVectorSize (Spline|GetTangentatDistanceAlongSpline _spline (* (+ _index 1) (Variables|Default|GetCalculatedSegmentLen)) "Local") 0.0 (Variables|Default|GetCalculatedSegmentLen)) true :!class /Script/Engine.SplineMeshComponent)))