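; MeshSpawner builds a wall-like grid of physics-simulated static mesh actors when play begins.
; Nested Rows and Cols loops on BeginPlay spawn movable StaticMeshActors with the chosen Mesh and a fixed mass override.
; GetTransformForRowAndCol offsets each from the spawner, by Height along Z and half of Distance per column along Y.
; That helper also prints each row and column, and always allows spawning.
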(event Collision|EventActorBeginOverlap
  (params (OtherActor :type Actor%20Object%20Reference)))

(event EventBeginPlay
  (while (!= (Variables|Default|GetCurrentRow) (Variables|Default|GetRows))
    (Utilities|FlowControl|Sequence
      (:then_0
        (while (!= (Variables|Default|GetCurrentCol) (Variables|Default|GetCols))
          (Utilities|FlowControl|Sequence
            (:then_0
              (if (.ShouldSpawn (CallFunction|GetTransformforRowandCol (Variables|Default|GetCurrentRow) (Variables|Default|GetCurrentCol)))
                (bind _returnvalue (Game|SpawnActorfromClass "/Script/Engine.StaticMeshActor" (.Transform (CallFunction|GetTransformforRowandCol (Variables|Default|GetCurrentRow) (Variables|Default|GetCurrentCol))) "AlwaysSpawn" 0 0))
                (Components|StaticMesh|SetStaticMesh (Variables|/Script/Engine.StaticMeshActor|GetStaticMeshComponent _returnvalue) (Variables|Default|GetMesh))
                (Transformation|SetMobility _returnvalue "Movable")
                (Physics|SetSimulatePhysics (Variables|/Script/Engine.StaticMeshActor|GetStaticMeshComponent _returnvalue) true)
                (Class|PrimitiveComponent|SetMassOverrideinKg (Variables|/Script/Engine.StaticMeshActor|GetStaticMeshComponent _returnvalue) "None" 1e+01 true)))
            (:then_1
              (Math|Integer|IncrementInt (Variables|Default|GetCurrentCol)))))
        (Variables|Default|SetCurrentCol 0))
      (:then_1
        (Math|Integer|IncrementInt (Variables|Default|GetCurrentRow))))))

(fn ConstructionScript)

(fn GetTransformforRowandCol
  (params (Row :type Integer) (Col :type Integer))
  (bind _distance (Variables|Default|GetDistance))
  (bind _returnvalue (* Col _distance))
  (Development|PrintString (Utilities|String|Append (Utilities|String|ToString(Integer) Row) ":" (Utilities|String|ToString(Integer) Col)))
  (return true (Math|Transform|MakeTransform (+ (Transformation|GetActorLocation) (Math|Vector|MakeVector 0.0 (- _returnvalue (/ _returnvalue 2.0)) (* Row (Variables|Default|GetHeight)))))))