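; BP_AdaptiveInput is a vehicle input modifier that adapts throttle and brake to slope and forward speed.
; It scales the parent class's results, reading nose-up pitch from the forward vector's dot product with world up.
; Throttle is reduced on level or downhill ground and as forward speed rises.
; Brake values above half are softened at low absolute speed unless the nose points uphill, using the larger of the slope and speed factors.
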(fn CalcThrottleInput
  (params (MovementComponent :type Modular%20Movement%20Component%20Object%20Reference) (DeltaTime :type Float%20%28single-precision%29) (RawInput :type Float%20%28single-precision%29) (RawBrakeInput :type Float%20%28single-precision%29) (RawSteeringInput :type Float%20%28single-precision%29))
  (bind _returnvalue (|CallParentFunction MovementComponent DeltaTime RawInput RawBrakeInput 0.0))
  (return (* _returnvalue (* (Math|Float|MapRangeClamped (Math|Vector|DotProduct (Transformation|GetActorForwardVector (Components|GetOwner MovementComponent)) "0.000000,0.000000,1.000000") 0.0 0.12 0.3 1.0) (Math|Float|MapRangeClamped (Math|Conversions|ToFloat(Integer) (Class|ModularVehicleFunctionLibrary|GetForwardSpeedKMH MovementComponent)) 0.0 6e+01 1.0 0.3)))))

(fn CalcBrakeInput
  (params (MovementComponent :type Modular%20Movement%20Component%20Object%20Reference) (DeltaTime :type Float%20%28single-precision%29) (RawBrakeInput :type Float%20%28single-precision%29) (RawThrottleInput :type Float%20%28single-precision%29))
  (bind _returnvalue (|CallParentFunction MovementComponent DeltaTime RawBrakeInput RawThrottleInput))
  (if (> _returnvalue 0.5)
    (return (* _returnvalue (Math|Float|Max(Float) (Math|Float|MapRangeClamped (Math|Vector|DotProduct (Transformation|GetActorForwardVector (Components|GetOwner MovementComponent)) "0.000000,0.000000,1.000000") 0.0 0.16 0.0 1.0) (Math|Float|MapRangeClamped (Math|Float|Absolute(Float) (Math|Conversions|ToFloat(Integer) (Class|ModularVehicleFunctionLibrary|GetForwardSpeedKMH MovementComponent))) 0.0 6e+01 0.05 1.0))))
    (else
      (return _returnvalue))))