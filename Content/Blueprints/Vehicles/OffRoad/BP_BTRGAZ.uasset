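; Drivable off-road BTR GAZ vehicle built on modular wheel movement, with its own on-screen OffroadUI.
; Construction snaps the four wheel components to skeletal mesh sockets.
; Tick smooths engine RPM ratio at two rates for audio RPM and turbo, and drives particle strength that peaks at mid RPM.
; Inputs toggle an underside camera with light, front-wheel drive force for 4WD with a change notification, and counter-steering rear wheels.
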(event EventBeginPlay
  (bind _returnvalue (UserInterface|CreateWidget "/Game/Blueprints/UI/OffroadUI.OffroadUI_C"))
  (Variables|Default|SetUI _returnvalue)
  (UserInterface|Viewport|AddtoViewport (Variables|Default|GetUI) 0)
  (Default|CallON4WDChange false))

(event Collision|EventActorBeginOverlap
  (params (OtherActor :type Actor%20Object%20Reference)))

(event EventTick
  (params (DeltaSeconds :type Float%20%28single-precision%29))
  (bind _modularmovement (Variables|Default|GetModularMovement))
  (bind _returnvalue (Class|ModularVehicleFunctionLibrary|GetEngineRpmRatio _modularmovement))
  (Variables|Default|SetCurrentRpmRatio (Math|Interpolation|FInterptoConstant (Variables|Default|GetCurrentRpmRatio) _returnvalue DeltaSeconds 1.0))
  (Variables|Default|SetCurrentTurboRatio (Math|Interpolation|FInterptoConstant (Variables|Default|GetCurrentTurboRatio) _returnvalue DeltaSeconds 0.5))
  (Audio|Parameter|SetFloatParameter (Variables|Default|GetAudio) "RPM" (Variables|Default|GetCurrentRpmRatio) :!class /Script/Engine.AudioComponent)
  (Audio|Parameter|SetFloatParameter (Variables|Default|GetAudio) "Turbo" (Variables|Default|GetCurrentTurboRatio) :!class /Script/Engine.AudioComponent)
  (Effects|Components|ParticleSystem|SetFloatParameter (Variables|Default|GetParticleSystem) "Strentgh" (- 1.0 (Math|Float|Absolute(Float) (- (* (Class|ModularVehicleFunctionLibrary|GetEngineRpmRatio (Variables|Default|GetModularMovement)) 2.0) 1.0)))))

(event EventUnpossessed
  (params (OldController :type Controller%20Object%20Reference))
  (Widget|RemovefromParent (Variables|Default|GetUI)))

(event Input|ActionEvents|InputActionSwitchCam
  (params (Key :type Key%20Structure :default "None"))
  (:Pressed
    (Components|Activation|ToggleActive (Variables|Default|GetCamera))
    (Components|Activation|ToggleActive (Variables|Default|GetUnderCamera))
    (Rendering|ToggleVisibility (Variables|Default|GetLightToSeeUnder) false)))

(event Input|ActionEvents|InputActionAction1
  (params (Key :type Key%20Structure :default "None"))
  (:Pressed
    (bind _isa (Utilities|FlowControl|FlipFlop)
      (:A
        _)
      (:B
        _))
    (Utilities|Struct|SetmembersinWheelState (Variables|/Script/ModularMovement.ModularWheel|GetWheelState (Variables|Default|GetFront%20Right)) _isa)
    (Utilities|Struct|SetmembersinWheelState (Variables|/Script/ModularMovement.ModularWheel|GetWheelState (Variables|Default|GetFront%20Left)) _isa)
    (Default|CallON4WDChange _isa)))

(event Input|ActionEvents|InputActionAction2
  (params (Key :type Key%20Structure :default "None"))
  (:Pressed
    (bind _isa (Utilities|FlowControl|FlipFlop)
      (:A
        (Utilities|Struct|SetmembersinWheelState (Variables|/Script/ModularMovement.ModularWheel|GetWheelState (Variables|Default|GetBack%20Right)) (select _isa -1.0 0.0) :!label _label)
        (Utilities|Struct|SetmembersinWheelState (Variables|/Script/ModularMovement.ModularWheel|GetWheelState (Variables|Default|GetBack%20Left)) (select _isa -1.0 0.0)))
      (:B
        (Utilities|FlowControl|Sequence
          (:then_0
            (goto _label))
          (:then_1
            (Class|ModularWheel|SetSteeronWheel (Variables|Default|GetBack%20Left) 0.0)))))))

(fn ConstructionScript
  (Transformation|SetRelativeLocation (Variables|Default|GetFront%20Right) (.location (Transformation|GetSocketTransform (Variables|Default|GetSkeletalMesh) "Wheel_FrontRight" "RTS_Actor")) false false)
  (Transformation|SetRelativeLocation (Variables|Default|GetFront%20Left) (.location (Transformation|GetSocketTransform (Variables|Default|GetSkeletalMesh) "Wheel_FrontLeft" "RTS_Actor")) false false)
  (Transformation|SetRelativeLocation (Variables|Default|GetBack%20Left) (.location (Transformation|GetSocketTransform (Variables|Default|GetSkeletalMesh) "Wheel_BackLeft" "RTS_Actor")) false false)
  (Transformation|SetRelativeLocation (Variables|Default|GetBack%20Right) (.location (Transformation|GetSocketTransform (Variables|Default|GetSkeletalMesh) "Wheel_BackRight" "RTS_Actor")) false false))