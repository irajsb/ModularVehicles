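; BP_BTR80 is the BTR-80 vehicle Blueprint, driving engine audio, particle effects and spring-arm camera behavior.
; Each tick it smooths the modular movement's engine RPM ratio at two rates into RPM and slower-lagging Turbo audio parameters.
; The raw ratio sets particle strength through a triangle curve peaking at mid RPM.
; Any input reported by BP_PlayerController sets a cooldown on the spring arm.
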(event Custom|HadAnyInput_Event_0
  (Class|VehicleSpringArm|SetCooldown (Variables|Default|GetVehicleSpringArm) 3.0))

(event EventBeginPlay
  (bind _asbp_player_controller (Utilities|Casting|CastToBP_PlayerController (Game|GetPlayerController 0)))
  (EventDispatchers|AssignHadAnyInput _asbp_player_controller (delegate Custom|HadAnyInput_Event_0)))

(event Collision|EventActorBeginOverlap
  (params (OtherActor :type Actor%20Object%20Reference)))

(event EventTick
  (params (DeltaSeconds :type Float%20%28single-precision%29))
  (bind _modularmovement (Variables|Default|GetModularMovement))
  (bind _returnvalue (Class|ModularVehicleFunctionLibrary|GetEngineRpmRatio _modularmovement))
  (Variables|Default|SetCurrentRpmRatio (Math|Interpolation|FInterptoConstant (Variables|Default|GetCurrentRpmRatio) _returnvalue DeltaSeconds 1.0))
  (Variables|Default|SetCurrentTurboRatio (Math|Interpolation|FInterptoConstant (Variables|Default|GetCurrentTurboRatio) _returnvalue DeltaSeconds 0.5))
  (Audio|Parameter|SetFloatParameter (Variables|Default|GetAudio) "RPM" (Variables|Default|GetCurrentRpmRatio) :!class /Script/Engine.AudioComponent)
  (Audio|Parameter|SetFloatParameter (Variables|Default|GetAudio) "Turbo" (Variables|Default|GetCurrentTurboRatio) :!class /Script/Engine.AudioComponent)
  (Effects|Components|ParticleSystem|SetFloatParameter (Variables|Default|GetParticleSystem) "Strentgh" (- 1.0 (Math|Float|Absolute(Float) (- (* (Class|ModularVehicleFunctionLibrary|GetEngineRpmRatio (Variables|Default|GetModularMovement)) 2.0) 1.0)))))

(fn ConstructionScript)