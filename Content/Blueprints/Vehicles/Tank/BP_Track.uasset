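; BP_Track is a tank track Blueprint that pairs a TankTrack component with the idlers and sprocket it visually turns.
; The construction script passes an ordered list of L, idler, Sway and sprocket components to TankTrack.SetupComponents.
; Each Tick pitches the four idlers and the sprocket by negated TrackSpeed over their radius, without delta-time scaling.
; The CorrectAngle angle-wrapping helper is left unconnected.
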(event EventBeginPlay)

(event Collision|EventActorBeginOverlap
  (params (OtherActor :type Actor%20Object%20Reference)))

(event EventTick
  (params (DeltaSeconds :type Float%20%28single-precision%29))
  (for _array_element (Utilities|Array|MakeArray (Variables|Default|GetIdlerL) (Variables|Default|GetIdlerL1) (Variables|Default|GetIdlerL2) (Variables|Default|GetIdlerL3) (Variables|Default|GetSprocketL))
    (Transformation|SetRelativeRotation _array_element (Math|Rotator|CombineRotators (Variables|/Script/Engine.SceneComponent|GetRelativeRotation _array_element) (Math|Rotator|MakeRotator 0.0 (Utilities|Operators|Divide (Variables|/Script/ModularMovement.TankTrackComponent|GetTrackSpeed (Variables|Default|GetTankTrack)) (Variables|/Script/ModularMovement.IdlerComponent|GetRadius _array_element) -1.0) 0.0)) false false)))

(fn ConstructionScript
  (Class|TankTrackComponent|SetupComponents (Variables|Default|GetTankTrack) (Utilities|Array|MakeArray (Variables|Default|GetL6) (Variables|Default|GetL5) (Variables|Default|GetL4) (Variables|Default|GetL3) (Variables|Default|GetL2) (Variables|Default|GetL1) (Variables|Default|GetIdlerL) (Variables|Default|GetSway1) (Variables|Default|GetIdlerL1) (Variables|Default|GetSway2) (Variables|Default|GetIdlerL2) (Variables|Default|GetSway3) (Variables|Default|GetIdlerL3) (Variables|Default|GetSprocketL))))

(fn CorrectAngle
  (params (In :type Float%20%28double-precision%29))
  (if (< In -9e+01)
    (return (+ In 1.8e+02))
    (elif (> In 9e+01)
      (return (- In 1.8e+02))
      (else
        (return In)))))