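; Player-drivable heavy tank with cannon, HUD, engine and track audio, and scrolling track materials driven by ModularMovement and wheel speeds.
; Once player-possessed, a camera trace sets a rate-limited, pitch-clamped CurrentAimRot, and a muzzle trace places the reticle widget at the predicted impact.
; Left click spawns a projectile with recoil impulse and effects, then gates firing during reload.
; The construction script snaps each ModularWheel to its name-matched mesh socket.
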(event Custom|UpdateSound
  (Audio|Parameter|SetFloatParameter (Variables|Default|GetTrackSound) "Speed" (/ (+ (Math|Float|Absolute(Float) (Class|ModularWheel|GetTrackSpeed (Variables|Default|GetR3))) (Math|Float|Absolute(Float) (Class|ModularWheel|GetTrackSpeed (Variables|Default|GetL3)))) 3e+03) :!class /Script/AudioExtensions.AudioParameterControllerInterface))

(event Custom|EngineSound
  (params (DeltaSeconds :type Float%20%28single-precision%29))
  (bind _returnvalue (* DeltaSeconds -0.02))
  (bind _mleft (Variables|Default|GetMLeft))
  (bind _modularmovement (Variables|Default|GetModularMovement))
  (bind _engineaudio (Variables|Default|GetEngineAudio))
  (bind _m_right (Variables|Default|GetM_Right))
  (Variables|Default|SetCurrentRpmRatio (Math|Interpolation|FInterptoConstant (Variables|Default|GetCurrentRpmRatio) (Class|ModularVehicleFunctionLibrary|GetEngineRpmRatio _modularmovement) DeltaSeconds 1.0))
  (Variables|Default|SetCurrentLoad (Math|Interpolation|FInterptoConstant (Variables|Default|GetCurrentLoad) (Variables|/Script/ModularMovement.ModularMovementComponent|GetThrottleInput _modularmovement) DeltaSeconds 5.0))
  (Audio|Parameter|SetFloatParameter _engineaudio "RPM" (Variables|Default|GetCurrentRpmRatio) :!class /Script/Engine.AudioComponent)
  (Audio|Parameter|SetFloatParameter _engineaudio "Load" 0.0 :!class /Script/Engine.AudioComponent)
  (bind _returnvalue_2 (Rendering|Material|GetScalarParameterValue _mleft "Offset" :!class /Script/Engine.MaterialInstanceDynamic))
  (Rendering|Material|SetScalarParameterValue _mleft "Offset" (Class|ModularWheel|GetTrackOffset (Variables|Default|GetL3) _returnvalue_2 _returnvalue) :!class /Script/Engine.MaterialInstanceDynamic)
  (bind _returnvalue_3 (Rendering|Material|GetScalarParameterValue _m_right "Offset" :!class /Script/Engine.MaterialInstanceDynamic))
  (Rendering|Material|SetScalarParameterValue _m_right "Offset" (Class|ModularWheel|GetTrackOffset (Variables|Default|GetR3) _returnvalue_3 _returnvalue) :!class /Script/Engine.MaterialInstanceDynamic))

(event EventBeginPlay
  (bind _skeletalmesh (Variables|Default|GetSkeletalMesh))
  (bind _returnvalue (UserInterface|CreateWidget "/Game/Blueprints/Vehicles/Tank/WB_TankUI.WB_TankUI_C"))
  (UserInterface|Viewport|AddtoViewport _returnvalue 0)
  (bind _returnvalue_2 (Rendering|Material|CreateDynamicMaterialInstance _skeletalmesh 1 "/Game/Art/Vehicles/Tank/Heavy/M_Track.M_Track" "None" :!class /Script/Engine.PrimitiveComponent))
  (Variables|Default|SetMLeft _returnvalue_2)
  (bind _returnvalue_3 (Rendering|Material|CreateDynamicMaterialInstance _skeletalmesh 2 "/Game/Art/Vehicles/Tank/Heavy/M_Track.M_Track" "None" :!class /Script/Engine.PrimitiveComponent))
  (Variables|Default|SetM_Right _returnvalue_3))

(event EventTick
  (params (DeltaSeconds :type Float%20%28single-precision%29))
  (bind _camera (Variables|Default|GetCamera))
  (bind _skeletalmesh (Variables|Default|GetSkeletalMesh))
  (bind _returnvalue (Transformation|GetWorldLocation _camera))
  (bind _returnvalue_2 (Transformation|GetSocketLocation _skeletalmesh "Tip"))
  (CallFunction|EngineSound DeltaSeconds)
  (CallFunction|UpdateSound)
  (Utilities|FlowControl|Gate true
    (:Exit
      (bind _outhit (Collision|LineTraceByChannel _returnvalue (+ _returnvalue (* (.WorldDirection (Class|GameplayStatics|DeprojectScreentoWorld (Game|GetPlayerController 0) (/ (Viewport|GetViewportSize) "(X=2.000000,Y=3.000000)"))) 1e+06)) "TraceTypeQuery1" false 0 "None"))
      (Variables|Default|SetCurrentAimRot (Math|Rotator|MakeRotator 0.0 (Math|Float|ClampAngle (.Pitch (Math|Rotator|BreakRotator (Class|KismetMathLibrary|RInterptoConstant (Variables|Default|GetCurrentAimRot) (Math|Rotator|CombineRotators (Math|Rotator|FindLookatRotation (Transformation|GetSocketLocation (Variables|Default|GetSkeletalMesh) "Tip") (select (.bblockinghit _outhit) (.impactpoint _outhit) (.traceend _outhit))) (Class|KismetMathLibrary|NegateRotator (Transformation|GetActorRotation))) DeltaSeconds 45.0))) -1e+01 3e+01) (.Yaw (Math|Rotator|BreakRotator (Class|KismetMathLibrary|RInterptoConstant (Variables|Default|GetCurrentAimRot) (Math|Rotator|CombineRotators (Math|Rotator|FindLookatRotation (Transformation|GetSocketLocation (Variables|Default|GetSkeletalMesh) "Tip") (select (.bblockinghit _outhit) (.impactpoint _outhit) (.traceend _outhit))) (Class|KismetMathLibrary|NegateRotator (Transformation|GetActorRotation))) DeltaSeconds 45.0)))))
      (bind _outhit_2 (Collision|LineTraceByChannel _returnvalue_2 (+ _returnvalue_2 (* (Math|Vector|GetForwardVector (Math|Rotator|CombineRotators (Variables|Default|GetCurrentAimRot) (Transformation|GetActorRotation))) 1e+15)) "TraceTypeQuery1" false 0 "None"))
      (Transformation|SetWorldLocation (Variables|Default|GetWidget) (Math|Vector|SelectVector (.impactpoint _outhit_2) (.traceend _outhit_2) (.bblockinghit _outhit_2)) false false))))

(event EventPossessed
  (params (NewController :type Controller%20Object%20Reference))
  (bind _camera (Variables|Default|GetCamera))
  (bind _skeletalmesh (Variables|Default|GetSkeletalMesh))
  (bind _returnvalue (Transformation|GetWorldLocation _camera))
  (bind _returnvalue_2 (Transformation|GetSocketLocation _skeletalmesh "Tip"))
  (if (Class|Controller|IsPlayerController NewController)
    (Utilities|FlowControl|Gate true) ; enters at Open
  ))

(event Input|ActionEvents|InputActionLeftMouse
  (params (Key :type Key%20Structure :default "None"))
  (bind _skeletalmesh (Variables|Default|GetSkeletalMesh))
  (bind _returnvalue (Transformation|GetSocketTransform _skeletalmesh "Tip" "RTS_World"))
  (bind (_location _rotation) (Math|Transform|BreakTransform _returnvalue))
  (bind (_location_2 _rotation_2) (Math|Transform|BreakTransform _returnvalue))
  (:Pressed
    (Utilities|FlowControl|Gate false :!label _label
      (:Exit
        (Utilities|FlowControl|Sequence
          (:then_0
            (bind _returnvalue_2 (Game|SpawnActorfromClass "/Game/Blueprints/Vehicles/Tank/Projectile/BP_Projectile.BP_Projectile_C" (Math|Transform|MakeTransform _location _rotation "2.000000,2.000000,2.000000") "AlwaysSpawn" "MultiplyWithRoot" 0 0))
            (Collision|IgnoreActorwhenMoving (Variables|/Game/Blueprints/Vehicles/Tank/Projectile/BP_Projectile.BP_Projectile_C|GetStaticMesh _returnvalue_2) self true)
            (Physics|AddImpulseatLocation (Variables|Default|GetSkeletalMesh) (* (Math|Vector|GetForwardVector _rotation_2) -5e+06) _location_2 "None")
            (Audio|PlaySoundatLocation "/Game/Art/Sound/SFX/Tank/cannon_40mm_l70_shot2_2_Cue.cannon_40mm_l70_shot2_2_Cue" _location_2 "0, 0, 0" 1.0 1.0 0.0 0 0 0 0)
            (Audio|PlaySoundatLocation "/Game/Art/Sound/SFX/Tank/Eject1_Cue.Eject1_Cue" "0, 0, 0" "0, 0, 0" 1.0 1.0 0.0 0 0 0 0)
            (Effects|SpawnEmitteratLocation "/Game/StarterContent/Particles/P_BarrelFlash.P_BarrelFlash" (Transformation|GetSocketLocation (Variables|Default|GetSkeletalMesh) "Tip") (Variables|Default|GetCurrentAimRot)))
          (:then_1
            (goto _label Close))
          (:then_2
            (Utilities|FlowControl|Delay 3.0)
            (Audio|PlaySoundatLocation "/Game/Art/Sound/SFX/Tank/Reload.Reload" (Transformation|GetWorldLocation (Variables|Default|GetSkeletalMesh)) "0, 0, 0" 1.0 1.0 0.0 0 0 0 0)
            (goto _label Open)))))))

(fn ConstructionScript
  (for _array_element (Actor|GetComponentsByClass "/Script/Engine.ActorComponent")
    (bind _asmodular_wheel (Utilities|Casting|CastToModularWheel _array_element))
    (Transformation|SetWorldLocation _asmodular_wheel (Transformation|GetSocketLocation (Variables|Default|GetSkeletalMesh) (Utilities|String|StringToName (.RightS (Utilities|String|Split (Utilities|GetDisplayName _array_element) ".")))) false false)))