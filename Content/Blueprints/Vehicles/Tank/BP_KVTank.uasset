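; Player-drivable KV tank that aims its turret with the camera and fires a cannon.
; Left click spawns a projectile with recoil impulse and effects, then a gate blocks firing until a timed reload ends.
; While player-possessed, Tick traces from the camera, rotates turret and pitch-clamped barrel toward the hit at constant speed, and places a reticle widget at the barrel's true aim point.
; The same tick drives engine and track audio from smoothed RPM, throttle and track speeds.
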(event Custom|UpdateSound
  (Audio|Parameter|SetFloatParameter (Variables|Default|GetTrackSound) "Speed" (/ (+ (Math|Float|Absolute(Float) (Variables|/Script/ModularMovement.TankTrackComponent|GetTrackSpeed (Variables|/Game/Blueprints/Vehicles/Tank/BP_Track.BP_Track_C|GetTankTrack (.AsBP%20Track (Utilities|Casting|CastToBP_Track (Variables|/Script/Engine.ChildActorComponent|GetChildActor (Variables|Default|GetChildActor))))))) (Math|Float|Absolute(Float) (Variables|/Script/ModularMovement.TankTrackComponent|GetTrackSpeed (Variables|/Game/Blueprints/Vehicles/Tank/BP_Track.BP_Track_C|GetTankTrack (.AsBP%20Track (Utilities|Casting|CastToBP_Track (Variables|/Script/Engine.ChildActorComponent|GetChildActor (Variables|Default|GetChildActor1)))))))) 3e+03) :!class /Script/AudioExtensions.AudioParameterControllerInterface))

(event Custom|EngineSound
  (params (DeltaSeconds :type Float%20%28single-precision%29))
  (bind _modularmovement (Variables|Default|GetModularMovement))
  (bind _engineaudio (Variables|Default|GetEngineAudio))
  (Variables|Default|SetCurrentRpmRatio (Math|Interpolation|FInterptoConstant (Variables|Default|GetCurrentRpmRatio) (Class|ModularVehicleFunctionLibrary|GetEngineRpmRatio _modularmovement) DeltaSeconds 1.0))
  (Variables|Default|SetCurrentLoad (Math|Interpolation|FInterptoConstant (Variables|Default|GetCurrentLoad) (Variables|/Script/ModularMovement.ModularMovementComponent|GetThrottleInput _modularmovement) DeltaSeconds 5.0))
  (Audio|Parameter|SetFloatParameter _engineaudio "RPM" (Variables|Default|GetCurrentRpmRatio) :!class /Script/Engine.AudioComponent)
  (Audio|Parameter|SetFloatParameter _engineaudio "Load" (Variables|Default|GetCurrentLoad) :!class /Script/Engine.AudioComponent))

(event EventBeginPlay
  (bind _returnvalue (UserInterface|CreateWidget "/Game/Blueprints/Vehicles/Tank/WB_TankUI.WB_TankUI_C"))
  (UserInterface|Viewport|AddtoViewport _returnvalue 0))

(event EventTick
  (params (DeltaSeconds :type Float%20%28single-precision%29))
  (bind _camera (Variables|Default|GetCamera))
  (bind _barrel (Variables|Default|GetBarrel))
  (bind _returnvalue (Transformation|GetWorldLocation _barrel))
  (bind _returnvalue_2 (Transformation|GetWorldLocation _camera))
  (Utilities|FlowControl|Gate true
    (:Exit
      (CallFunction|EngineSound DeltaSeconds)
      (CallFunction|UpdateSound)
      (bind _outhit (Collision|LineTraceByChannel _returnvalue_2 (+ _returnvalue_2 (* (.WorldDirection (Class|GameplayStatics|DeprojectScreentoWorld (Game|GetPlayerController 0) (/ (Viewport|GetViewportSize) "(X=2.000000,Y=3.000000)"))) 1e+06)) "TraceTypeQuery1" false 0 "None"))
      (Transformation|SetRelativeRotation (Variables|Default|GetTurret) (Math|Rotator|MakeRotator 0.0 0.0 (.Yaw (Math|Rotator|BreakRotator (Class|KismetMathLibrary|RInterptoConstant (Math|Rotator|MakeRotator 0.0 (.Pitch (Math|Rotator|BreakRotator (Variables|/Script/Engine.SceneComponent|GetRelativeRotation (Variables|Default|GetBarrel)))) (.Yaw (Math|Rotator|BreakRotator (Variables|/Script/Engine.SceneComponent|GetRelativeRotation (Variables|Default|GetTurret))))) (Math|Rotator|CombineRotators (Math|Rotator|FindLookatRotation (Transformation|GetWorldLocation (Variables|Default|GetBarrel)) (select (.bblockinghit _outhit) (.impactpoint _outhit) (.traceend _outhit))) (Class|KismetMathLibrary|NegateRotator (Transformation|GetActorRotation))) DeltaSeconds 3e+01)))) false false)
      (Transformation|SetRelativeRotation (Variables|Default|GetBarrel) (Math|Rotator|MakeRotator 0.0 (Math|Float|ClampAngle (.Pitch (Math|Rotator|BreakRotator (Class|KismetMathLibrary|RInterptoConstant (Math|Rotator|MakeRotator 0.0 (.Pitch (Math|Rotator|BreakRotator (Variables|/Script/Engine.SceneComponent|GetRelativeRotation (Variables|Default|GetBarrel)))) (.Yaw (Math|Rotator|BreakRotator (Variables|/Script/Engine.SceneComponent|GetRelativeRotation (Variables|Default|GetTurret))))) (Math|Rotator|CombineRotators (Math|Rotator|FindLookatRotation (Transformation|GetWorldLocation (Variables|Default|GetBarrel)) (select (.bblockinghit _outhit) (.impactpoint _outhit) (.traceend _outhit))) (Class|KismetMathLibrary|NegateRotator (Transformation|GetActorRotation))) DeltaSeconds 3e+01))) -1e+01 3e+01) 0.0) false false)
      (bind _outhit_2 (Collision|LineTraceByChannel _returnvalue (+ _returnvalue (* (Math|Vector|GetForwardVector (Variables|Default|GetBarrel)) 1e+15)) "TraceTypeQuery1" false 0 "None"))
      (Transformation|SetWorldLocation (Variables|Default|GetWidget) (Math|Vector|SelectVector (.impactpoint _outhit_2) (.traceend _outhit_2) (.bblockinghit _outhit_2)) false false))))

(event EventPossessed
  (params (NewController :type Controller%20Object%20Reference))
  (bind _camera (Variables|Default|GetCamera))
  (bind _barrel (Variables|Default|GetBarrel))
  (bind _returnvalue (Transformation|GetWorldLocation _barrel))
  (bind _returnvalue_2 (Transformation|GetWorldLocation _camera))
  (if (Class|Controller|IsPlayerController NewController)
    (Rendering|SetVisibility (Variables|Default|GetWidget) true false)
    (Utilities|FlowControl|Gate true) ; enters at Open
  ))

(event EventUnpossessed
  (params (OldController :type Controller%20Object%20Reference))
  (bind _camera (Variables|Default|GetCamera))
  (bind _barrel (Variables|Default|GetBarrel))
  (bind _returnvalue (Transformation|GetWorldLocation _barrel))
  (bind _returnvalue_2 (Transformation|GetWorldLocation _camera))
  (Utilities|FlowControl|Gate true) ; enters at Close
)

(event Input|ActionEvents|InputActionLeftMouse
  (params (Key :type Key%20Structure :default "None"))
  (bind _tip (Variables|Default|GetTip))
  (bind _tip_2 (Variables|Default|GetTip))
  (bind _returnvalue (Transformation|GetWorldLocation _tip))
  (:Pressed
    (Utilities|FlowControl|Gate false :!label _label
      (:Exit
        (Utilities|FlowControl|Sequence
          (:then_0
            (bind _returnvalue_2 (Game|SpawnActorfromClass "/Game/Blueprints/Vehicles/Tank/Projectile/BP_Projectile.BP_Projectile_C" (Transformation|GetWorldTransform _tip) "AlwaysSpawn" "MultiplyWithRoot" 0 0))
            (Collision|IgnoreActorwhenMoving (Variables|/Game/Blueprints/Vehicles/Tank/Projectile/BP_Projectile.BP_Projectile_C|GetStaticMesh _returnvalue_2) self true)
            (Physics|AddImpulseatLocation (Variables|Default|GetStaticMesh) (* (Math|Vector|GetForwardVector _tip) -5e+05) _returnvalue "None")
            (Audio|PlaySoundatLocation "/Game/Art/Sound/SFX/Tank/cannon_40mm_l70_shot2_2_Cue.cannon_40mm_l70_shot2_2_Cue" _returnvalue "0, 0, 0" 1.0 1.0 0.0 0 0 0 0)
            (Audio|PlaySoundatLocation "/Game/Art/Sound/SFX/Tank/Eject1_Cue.Eject1_Cue" "0, 0, 0" "0, 0, 0" 1.0 1.0 0.0 0 0 0 0)
            (Effects|SpawnEmitteratLocation "/Game/StarterContent/Particles/P_BarrelFlash.P_BarrelFlash" (Transformation|GetWorldLocation _tip_2) (Transformation|GetWorldRotation _tip_2)))
          (:then_1
            (goto _label Close))
          (:then_2
            (Utilities|FlowControl|Delay 3.0)
            (Audio|PlaySoundatLocation "/Game/Art/Sound/SFX/Tank/Reload.Reload" (Transformation|GetWorldLocation (Variables|Default|GetStaticMesh)) "0, 0, 0" 1.0 1.0 0.0 0 0 0 0)
            (goto _label Open)))))))

(fn ConstructionScript)