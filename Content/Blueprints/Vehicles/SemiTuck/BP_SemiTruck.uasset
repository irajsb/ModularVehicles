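; BP_SemiTruck is a drivable semi truck that can hitch trailers.
; Each tick, smoothed engine RPM ratios drive engine and turbo audio plus particle strength, which peaks at mid RPM.
; A sphere trace at the hitch socket finds nearby trailers, showing a prompt and opening a gate for Action2.
; Attaching constrains the trailer to the truck, enables its physics and passes its wheels to ModularMovement.
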(event Custom|CheckForAttach
  (bind _attachsocket (Variables|Default|GetAttachSocket))
  (bind _returnvalue (Transformation|GetWorldLocation _attachsocket))
  (if (not (Variables|Default|GetIsAttached))
    (bind _outhit (Collision|SphereTraceByChannel _returnvalue _returnvalue 5e+01 "TraceTypeQuery1" false 0 "None"))
    (bind _astrailer (Utilities|Casting|CastToTrailer (.HitActor (Collision|BreakHitResult _outhit))))
    (Variables|Default|SetTrailer (.HitActor (Collision|BreakHitResult _outhit)))
    (if (< (Math|Vector|VectorLength (- _returnvalue (Transformation|GetWorldLocation (Variables|/Game/Blueprints/Vehicles/SemiTuck/Trailer.Trailer_C|GetAttachSocket _astrailer)))) 5e+01)
      (Utilities|FlowControl|Sequence
        (:then_0
          (Utilities|IsValid (Variables|Default|GetAttach)
            (:Is%20Not%20Valid
              (bind _returnvalue_2 (UserInterface|CreateWidget "/Game/Blueprints/Vehicles/SemiTuck/WB_AttachMessage.WB_AttachMessage_C"))
              (bind _output_get (Variables|Default|SetAttach _returnvalue_2))
              (UserInterface|Viewport|AddtoViewport _output_get 0))))
        (:then_1
          (Utilities|FlowControl|Gate true) ; enters at Open
        ))
      (else
        (Utilities|FlowControl|Sequence
          (:then_0
            (Utilities|FlowControl|Gate true) ; enters at Close
          )
          (:then_1
            (bind _attach (Variables|Default|GetAttach)
              (:then
                (Widget|RemovefromParent _attach)
                (Variables|Default|SetAttach 0))
              (:else))))))))

(event Custom|HadAnyInput_Event_0
  (Class|VehicleSpringArm|SetCooldown (Variables|Default|GetVehicleSpringArm) 3.0))

(event EventBeginPlay
  (bind _asbp_player_controller (Utilities|Casting|CastToBP_PlayerController (Game|GetPlayerController 0)))
  (EventDispatchers|AssignHadAnyInput _asbp_player_controller (delegate Custom|HadAnyInput_Event_0)))

(event EventTick
  (params (DeltaSeconds :type Float%20%28single-precision%29))
  (bind _modularmovement (Variables|Default|GetModularMovement))
  (bind _returnvalue (Class|ModularVehicleFunctionLibrary|GetEngineRpmRatio _modularmovement))
  (Variables|Default|SetCurrentRpmRatio (Math|Interpolation|FInterptoConstant (Variables|Default|GetCurrentRpmRatio) _returnvalue DeltaSeconds 1.0))
  (Variables|Default|SetCurrentTurboRatio (Math|Interpolation|FInterptoConstant (Variables|Default|GetCurrentTurboRatio) _returnvalue DeltaSeconds 0.5))
  (Audio|Parameter|SetFloatParameter (Variables|Default|GetAudio) "RPM" (Variables|Default|GetCurrentRpmRatio) :!class /Script/Engine.AudioComponent)
  (Audio|Parameter|SetFloatParameter (Variables|Default|GetAudio) "Turbo" (Variables|Default|GetCurrentTurboRatio) :!class /Script/Engine.AudioComponent)
  (Effects|Components|ParticleSystem|SetFloatParameter (Variables|Default|GetParticleSystem) "Strentgh" (- 1.0 (Math|Float|Absolute(Float) (- (* (Class|ModularVehicleFunctionLibrary|GetEngineRpmRatio (Variables|Default|GetModularMovement)) 2.0) 1.0))))
  (CallFunction|CheckforAttach))

(event Input|ActionEvents|InputActionAction2
  (params (Key :type Key%20Structure :default "None"))
  (:Pressed
    (Utilities|FlowControl|Gate true
      (:Exit
        (Widget|RemovefromParent (Variables|Default|GetAttach))
        (Variables|Default|SetIsAttached true)
        (bind _astrailer (Utilities|Casting|CastToTrailer (Variables|Default|GetTrailer)))
        (Class|PhysicsConstraintComponent|SetConstrainedComponents (Variables|/Game/Blueprints/Vehicles/SemiTuck/Trailer.Trailer_C|GetPhysicsConstraint _astrailer) (Variables|Default|GetStaticMesh) "None" (Variables|/Game/Blueprints/Vehicles/SemiTuck/Trailer.Trailer_C|GetStaticMesh _astrailer) "None")
        (Physics|SetSimulatePhysics (Variables|/Game/Blueprints/Vehicles/SemiTuck/Trailer.Trailer_C|GetStaticMesh _astrailer) true)
        (Class|ModularMovementComponent|UpdateComponents (Variables|Default|GetModularMovement) (Default|GetWheels _astrailer))))))

(fn ConstructionScript)