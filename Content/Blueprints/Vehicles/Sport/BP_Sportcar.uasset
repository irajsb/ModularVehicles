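; BP_Sportcar is a drivable sports car Blueprint with cosmetic audio, exhaust effects and a local HUD.
; BeginPlay adds the SportUI widget for the local player and hooks player input to a spring-arm camera cooldown.
; Tick smooths engine RPM ratio from ModularMovement into RPM and Turbo audio parameters at different rates.
; ExhaustFlash fires particles and a flutter sound, while a debug key binds gear-change timing printouts.
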(event Custom|ExhaustFlash
  (Components|Activation|Activate (Variables|Default|GetP_Flash1) true)
  (Audio|SpawnSoundAttached "/Game/Art/Sound/SFX/SC_Flutter.SC_Flutter" (Variables|Default|GetStaticMesh) "None" "0, 0, 0" "0, 0, 0" "KeepRelativeOffset" false 0.1 1.0 0.0 0 0))

(event Custom|HadAnyInput_Event_0
  (Class|VehicleSpringArm|SetCooldown (Variables|Default|GetVehicleSpringArm) 3.0))

(event Custom|OnGearChange_Event_0
  (params (CurrentGear :type Integer) (TargetGear :type Integer) (Finished :type Boolean))
  (Development|PrintString (Utilities|String|ToString(Float) (Class|KismetMathLibrary|GetTotalMilliseconds (- (Math|DateTime|Now) (Variables|Default|GetTime)))) true true "(R=1.000000,G=0.219430,B=0.000000,A=1.000000)"))

(event EventBeginPlay
  (bind _returnvalue (Game|GetPlayerController 0))
  (if (Networking|IsDedicatedServer)
    (Networking|SwitchHasAuthority
      (:Remote
        _)))
  (if (Pawn|IsLocalPlayerController _returnvalue)
    (bind _returnvalue_2 (UserInterface|CreateWidget "/Game/Blueprints/UI/SportCar/SportUI.SportUI_C" _returnvalue))
    (UserInterface|Viewport|AddtoViewport _returnvalue_2 0)
    (EventDispatchers|AssignHadAnyInput (.AsBP%20Player%20Controller (Utilities|Casting|CastToBP_PlayerController (Game|GetPlayerController 0))) (delegate Custom|HadAnyInput_Event_0))))

(event Collision|EventActorBeginOverlap
  (params (OtherActor :type Actor%20Object%20Reference)))

(event EventTick
  (params (DeltaSeconds :type Float%20%28single-precision%29))
  (bind _modularmovement (Variables|Default|GetModularMovement))
  (bind _audio (Variables|Default|GetAudio))
  (bind _returnvalue (Class|ModularVehicleFunctionLibrary|GetEngineRpmRatio _modularmovement))
  (Variables|Default|SetCurrentRPMRatioCosmetic (Math|Interpolation|FInterptoConstant (Variables|Default|GetCurrentRPMRatioCosmetic) _returnvalue DeltaSeconds 1.0))
  (Variables|Default|SetCurrentTurboCosmetic (Math|Interpolation|FInterptoConstant (Variables|Default|GetCurrentTurboCosmetic) _returnvalue DeltaSeconds 0.5))
  (Audio|Parameter|SetFloatParameter _audio "RPM" (* (Variables|Default|GetCurrentRPMRatioCosmetic) 1e+02) :!class /Script/Engine.AudioComponent)
  (Audio|Parameter|SetFloatParameter _audio "Turbo" (Variables|Default|GetCurrentTurboCosmetic) :!class /Script/Engine.AudioComponent))

(event Input|KeyboardEvents|O
  (params (Key :type Key%20Structure :default "None"))
  (:Pressed
    (EventDispatchers|BindEventtoOnGearChange (Variables|Default|GetModularMovement) (delegate Custom|OnGearChange_Event_0))
    (Variables|Default|SetTime (Math|DateTime|Now))
    (Development|PrintString "Hello")))

(fn ConstructionScript)