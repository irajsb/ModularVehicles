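; AI sport car Blueprint that wanders endlessly, using AIMoveTo toward random reachable points nearby and picking a new one on arrival or after a failed attempt.
; Tick smooths the ModularMovement RPM ratio at two rates to drive RPM and Turbo audio parameters.
; For a local player it also creates the SportUI widget and puts the spring arm on cooldown upon input.
; Debug aids draw the target point and print gear-change timing.
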(event Custom|ExhaustFlash)

(event Custom|HadAnyInput_Event_0
  (Class|VehicleSpringArm|SetCooldown (Variables|Default|GetVehicleSpringArm) 3.0))

(event Custom|FindPoint
  (bind _output_get (Variables|Default|SetRandom%20Location (.RandomLocation (AI|Navigation|GetRandomReachablePointinRadius (Transformation|GetActorLocation) 3e+03 0 0))))
  (AI|AIMoveTo self _output_get 0 3e+02 false
    (:OnSuccess
      _)
    (:OnFail
      (Utilities|FlowControl|Delay 1.0)))
  (CallFunction|FindPoint))

(event Custom|OnGearChange_Event_0
  (params (CurrentGear :type Integer) (TargetGear :type Integer) (Finished :type Boolean))
  (Development|PrintString (Utilities|String|ToString(Float) (Class|KismetMathLibrary|GetTotalMilliseconds (- (Math|DateTime|Now) (Variables|Default|GetTime)))) true true "(R=1.000000,G=0.219430,B=0.000000,A=1.000000)"))

(event EventBeginPlay
  (bind _returnvalue (Game|GetPlayerController 0))
  (CallFunction|FindPoint)
  (if (Networking|IsDedicatedServer)
    (Networking|SwitchHasAuthority
      (:Remote
        _)))
  (if (Pawn|IsLocalPlayerController _returnvalue)
    (bind _returnvalue_2 (UserInterface|CreateWidget "/Game/Blueprints/UI/SportCar/SportUI.SportUI_C" _returnvalue))
    (UserInterface|Viewport|AddtoViewport _returnvalue_2 0)
    (EventDispatchers|AssignHadAnyInput (.AsBP%20Player%20Controller (Utilities|Casting|CastToBP_PlayerController (Game|GetPlayerController 0))) (delegate Custom|HadAnyInput_Event_0))))

(event Collision|EventActorBeginOverlap
  (params (OtherActor :type Actor%20Object%20Reference)))

(event EventTick
  (params (DeltaSeconds :type Float%20%28single-precision%29))
  (bind _modularmovement (Variables|Default|GetModularMovement))
  (bind _audio (Variables|Default|GetAudio))
  (bind _returnvalue (Class|ModularVehicleFunctionLibrary|GetEngineRpmRatio _modularmovement))
  (Utilities|FlowControl|Sequence
    (:then_0
      (Variables|Default|SetCurrentRPMRatioCosmetic (Math|Interpolation|FInterptoConstant (Variables|Default|GetCurrentRPMRatioCosmetic) _returnvalue DeltaSeconds 1.0))
      (Variables|Default|SetCurrentTurboCosmetic (Math|Interpolation|FInterptoConstant (Variables|Default|GetCurrentTurboCosmetic) _returnvalue DeltaSeconds 0.5))
      (Audio|Parameter|SetFloatParameter _audio "RPM" (* (Variables|Default|GetCurrentRPMRatioCosmetic) 1e+02) :!class /Script/Engine.AudioComponent)
      (Audio|Parameter|SetFloatParameter _audio "Turbo" (Variables|Default|GetCurrentTurboCosmetic) :!class /Script/Engine.AudioComponent))
    (:then_2
      (Rendering|Debug|DrawDebugSphere (Variables|Default|GetRandom%20Location) 1e+02 30 "(R=1.000000,G=0.080058,B=0.000000,A=1.000000)" 0.0))))

(event Input|KeyboardEvents|O
  (params (Key :type Key%20Structure :default "None"))
  (:Pressed
    (EventDispatchers|BindEventtoOnGearChange (Variables|Default|GetModularMovement) (delegate Custom|OnGearChange_Event_0))
    (Variables|Default|SetTime (Math|DateTime|Now))
    (Development|PrintString "Hello")))

(fn ConstructionScript)