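; Player controller that drives the controlled pawn as a modular vehicle and turns the player's view.
; Forward and Right axes feed the vehicle's throttle and steer inputs, while LookYaw and LookPitch add controller yaw and pitch.
; HandBrake press and release share one call that sets the brake from the key's current down state.
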(event EventBeginPlay)

(event EventTick
  (params (DeltaSeconds :type Float%20%28single-precision%29)))

(event Input|ActionEvents|InputActionHandBrake
  (params (Key :type Key%20Structure :default "None"))
  (:Pressed
    (Class|ModularVehicleFunctionLibrary|SetHandBrakeInputonModularVehicle (Pawn|GetControlledPawn) (Game|Player|IsInputKeyDown Key) :!label _label))
  (:Released
    (goto _label)))

(event Input|AxisEvents|InputAxisLookYaw
  (params (AxisValue :type Float%20%28single-precision%29))
  (Class|PlayerController|AddYawInput AxisValue))

(event Input|AxisEvents|InputAxisLookPitch
  (params (AxisValue :type Float%20%28single-precision%29))
  (Class|PlayerController|AddPitchInput AxisValue))

(event Input|AxisEvents|InputAxisForward
  (params (AxisValue :type Float%20%28single-precision%29))
  (Class|ModularVehicleFunctionLibrary|SetThrottleInputonModularVehicle (Pawn|GetControlledPawn) AxisValue))

(event Input|AxisEvents|InputAxisRight
  (params (AxisValue :type Float%20%28single-precision%29))
  (Class|ModularVehicleFunctionLibrary|SetSteerInputonModularVehicle (Pawn|GetControlledPawn) AxisValue))

(fn ConstructionScript)