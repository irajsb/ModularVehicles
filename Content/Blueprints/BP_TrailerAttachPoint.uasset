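; BP_TrailerAttachPoint shows and hides an on-screen attach message for a trailer attach point.
; On BeginPlay, only non-trailer instances bind to the OnTrailerPromptShow dispatcher.
; The handler lazily creates a WB_AttachMessage widget on first show, then reuses it by toggling visibility.
; The detach-prompt flag passed by the event is unused.
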(event Custom|OnTrailerPromptShow_Event
  (params (NewVisibility :type Boolean) (ShouldShowDeattachPrompt :type Boolean))
  (if NewVisibility
    (bind _attachwidget (Variables|Default|GetAttachWidget)
      (:then
        (Widget|SetVisibility _attachwidget "Visible"))
      (:else
        (bind _returnvalue (UserInterface|CreateWidget "/Game/Blueprints/Vehicles/SemiTuck/WB_AttachMessage.WB_AttachMessage_C"))
        (Variables|Default|SetAttachWidget _returnvalue)
        (UserInterface|Viewport|AddtoViewport _returnvalue 0)))
    (else
      (bind _attachwidget_2 (Variables|Default|GetAttachWidget)
        (:then
          (Widget|SetVisibility _attachwidget_2 "Hidden"))
        (:else)))))

(event EventBeginPlay
  (if (not (Variables|Default|GetIsTrailer))
    (EventDispatchers|AssignOnTrailerPromptShow (delegate Custom|OnTrailerPromptShow_Event))))